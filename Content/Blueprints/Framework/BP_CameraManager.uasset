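; BP_CameraManager is a camera manager that publishes the current camera state to the MPC_Camera material parameter collection.
; Every Tick it writes the camera location and the forward and right vectors from the camera rotation as vector parameters.
; It also writes a scalar Velocity parameter, which holds the speed of player pawn 0 rather than that of the camera.
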(event EventTick
  (params (DeltaSeconds :type Float%20%28single-precision%29))
  (bind _returnvalue (Camera|GetCameraLocation))
  (bind _returnvalue_2 (Camera|GetCameraRotation))
  (bind _returnvalue_3 (Math|Vector|GetForwardVector _returnvalue_2))
  (bind _returnvalue_4 (Math|Vector|GetRightVector _returnvalue_2))
  (Rendering|Material|SetVectorParameterValue "/Game/Materials/MPC_Camera.MPC_Camera" "Position" (Utilities|Struct|MakeLinearColor (.x _returnvalue) (.y _returnvalue) (.z _returnvalue) 1.0) :!class /Script/Engine.KismetMaterialLibrary)
  (Rendering|Material|SetVectorParameterValue "/Game/Materials/MPC_Camera.MPC_Camera" "Forward" (Utilities|Struct|MakeLinearColor (.x _returnvalue_3) (.y _returnvalue_3) (.z _returnvalue_3) 1.0) :!class /Script/Engine.KismetMaterialLibrary)
  (Rendering|Material|SetVectorParameterValue "/Game/Materials/MPC_Camera.MPC_Camera" "Right" (Utilities|Struct|MakeLinearColor (.x _returnvalue_4) (.y _returnvalue_4) (.z _returnvalue_4) 1.0) :!class /Script/Engine.KismetMaterialLibrary)
  (Rendering|Material|SetScalarParameterValue "/Game/Materials/MPC_Camera.MPC_Camera" "Velocity" (Math|Vector|VectorLength (Transformation|GetVelocity (Game|Player|GetPlayerPawn 0))) :!class /Script/Engine.KismetMaterialLibrary))

(fn ConstructionScript)