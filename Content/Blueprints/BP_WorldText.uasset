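; BP_WorldText is an actor that displays configurable text in the world through a widget component using WBP3D_FloatingText.
; The construction script applies the Hidden flag, sets the widget's draw size from Size and pushes Text into the widget.
; ShowText unhides the actor in game and reapplies the text.
; Both reach the widget through a GetWidget helper that casts it to the floating text class.
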(fn ConstructionScript
  (Rendering|SetActorHiddenInGame (Variables|Settings|GetHidden))
  (Class|WidgetComponent|SetDrawSize (Variables|Default|GetWidget) (Variables|Settings|GetSize))
  (bind _widgetref (Utilities|GetWidget))
  (Default|OverrideText _widgetref (Variables|Settings|GetText)))

(fn ShowText
  (Rendering|SetActorHiddenInGame false)
  (bind _widgetref (Utilities|GetWidget))
  (Default|OverrideText _widgetref (Variables|Settings|GetText)))