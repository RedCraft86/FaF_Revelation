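; Adapter Blueprint that applies a settings struct to an Ultra Dynamic Sky actor and its linked Ultra Dynamic Weather.
; ApplySettings sets night, fog and sky light levels, changes sky mode (every cloud type maps to the same enumerator) and snaps time of day.
; If weather is valid, it sets visibility and volume, then fades to a preset resolved from a gameplay tag by SelectWeather, defaulting to thick fog.
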(event EventApplySettings
  (params (UDSActor :type Actor%20Object%20Reference) (InSettings :type UDS%20Settings%20Structure%20%28by%20ref%29))
  (bind (_nightbrightness _fogbrightness _skylightintensity _cloudtype _timeofday _bweatherhidden _weathervolume _weatherfadetime _weatherpreset) (Utilities|Struct|BreakUDSSettings InSettings))
  (bind _asultra_dynamic_sky (Utilities|Casting|CastToUltra_Dynamic_Sky UDSActor))
  (Variables|/Game/AssetPacks/Effects/UltraDynamicSky/Blueprints/Ultra_Dynamic_Sky.Ultra_Dynamic_Sky_C|SetNight%20Brightness _asultra_dynamic_sky _nightbrightness)
  (Variables|/Game/AssetPacks/Effects/UltraDynamicSky/Blueprints/Ultra_Dynamic_Sky.Ultra_Dynamic_Sky_C|SetFog%20Color%20Intensity%20Scale _asultra_dynamic_sky _fogbrightness)
  (Variables|/Game/AssetPacks/Effects/UltraDynamicSky/Blueprints/Ultra_Dynamic_Sky.Ultra_Dynamic_Sky_C|SetSky%20Light%20Intensity _asultra_dynamic_sky _skylightintensity)
  (Default|ChangeSkyModeatRuntime _asultra_dynamic_sky (Utilities|Select :Index _cloudtype :Volumetric "NewEnumerator0" :Dynamic2D "NewEnumerator0" :None "NewEnumerator0"))
  (Default|TransitionTimeOfDay _asultra_dynamic_sky _timeofday 0.0 "Step" 0.0 true)
  (bind _ultra_dynamic_weather (Variables|/Game/AssetPacks/Effects/UltraDynamicSky/Blueprints/Ultra_Dynamic_Sky.Ultra_Dynamic_Sky_C|GetUltra%20Dynamic%20Weather _asultra_dynamic_sky)
    (:then
      (Rendering|SetActorHiddenInGame _ultra_dynamic_weather _bweatherhidden)
      (Default|SetMasterVolume _ultra_dynamic_weather _weathervolume)
      (Default|ChangeWeather _ultra_dynamic_weather (CallFunction|SelectWeather _weatherpreset) _weatherfadetime))
    (:else)))

(fn SelectWeather
  (params (Preset :type Gameplay%20Tag%20Structure))
  (|SwitchGameplayTag Preset
    (:Default
      (return "/Game/AssetPacks/Effects/UltraDynamicSky/Blueprints/Weather_Effects/Weather_Presets/Fog_Thick.Fog_Thick"))
    (:Weather.ClearSkies
      (return "/Game/AssetPacks/Effects/UltraDynamicSky/Blueprints/Weather_Effects/Weather_Presets/Clear_Skies.Clear_Skies"))
    (:Weather.Cloudy
      (return "/Game/AssetPacks/Effects/UltraDynamicSky/Blueprints/Weather_Effects/Weather_Presets/Cloudy.Cloudy"))
    (:Weather.FogThick
      (return "/Game/AssetPacks/Effects/UltraDynamicSky/Blueprints/Weather_Effects/Weather_Presets/Fog_Thick.Fog_Thick"))
    (:Weather.FogThin
      (return "/Game/AssetPacks/Effects/UltraDynamicSky/Blueprints/Weather_Effects/Weather_Presets/Fog_Thin.Fog_Thin"))
    (:Weather.Overcast
      (return "/Game/AssetPacks/Effects/UltraDynamicSky/Blueprints/Weather_Effects/Weather_Presets/Overcast.Overcast"))
    (:Weather.PartlyCloudy
      (return "/Game/AssetPacks/Effects/UltraDynamicSky/Blueprints/Weather_Effects/Weather_Presets/Partly_Cloudy.Partly_Cloudy"))
    (:Weather.Rain
      (return "/Game/AssetPacks/Effects/UltraDynamicSky/Blueprints/Weather_Effects/Weather_Presets/Rain.Rain"))
    (:Weather.RainFoggy
      (return "/Game/AssetPacks/Effects/UltraDynamicSky/Blueprints/Weather_Effects/Weather_Presets/Rain_Foggy.Rain_Foggy"))
    (:Weather.RainLight
      (return "/Game/AssetPacks/Effects/UltraDynamicSky/Blueprints/Weather_Effects/Weather_Presets/Rain_Light.Rain_Light"))
    (:Weather.Thunderstorm
      (return "/Game/AssetPacks/Effects/UltraDynamicSky/Blueprints/Weather_Effects/Weather_Presets/Rain_Thunderstorm.Rain_Thunderstorm"))))