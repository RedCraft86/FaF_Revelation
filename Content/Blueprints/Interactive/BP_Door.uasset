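; Interactive hinged door that extends a parent open/close actor, with a configurable mesh, materials, offset and open angle.
; State changes toggle Pawn and Vehicle blocking and, on opening, pick the target angle, mirrored by the last interactor's side when MultiAngle is set.
; CurvePlayer's evaluated value interpolates the pivot's yaw toward that angle.
; The construction script applies the mesh data and draws editor wire arcs previewing the swing.
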(event OnEvaluateTickBP(CurvePlayer)
  (params (Value :type Float%20%28single-precision%29) (Time :type Float%20%28single-precision%29))
  (Transformation|SetRelativeRotation (Variables|Default|GetDoorPivot) (Math|Rotator|MakeRotator 0.0 0.0 (Math|Float|Lerp 0.0 (Variables|Default|GetTargetAngle) Value)) false false))

(event EventOpenStateChanged
  (params (bState :type Boolean) (bImmediate :type Boolean))
  (bind _returnvalue (select bState "ECR_Ignore" "ECR_Block"))
  (bind _openangle (Variables|Settings|GetOpenAngle))
  (bind _doormesh (Variables|Default|GetDoorMesh))
  (|CallParentFunction bState bImmediate)
  (Collision|SetCollisionResponsetoChannel _doormesh "ECC_Vehicle" _returnvalue)
  (Collision|SetCollisionResponsetoChannel _doormesh "ECC_Pawn" _returnvalue)
  (if bState
    (if (Variables|Settings|GetMultiAngle)
      (Variables|Default|SetTargetAngle (select (Class|ToroMathLibrary|IsActorinFront 0 (Class|DoorBase|GetLastInteractor)) _openangle (* _openangle -1.0)))
      (else
        (Variables|Default|SetTargetAngle (Variables|Settings|GetOpenAngle))))))

(fn ConstructionScript
  (bind _doormesh (Variables|Default|GetDoorMesh))
  (bind _door (Variables|Settings|GetDoor))
  (Class|ToroPrimitiveUtils|FillMaterials _door)
  (Class|ToroPrimitiveUtils|SetStaticMeshData _doormesh _door)
  (Transformation|SetRelativeTransform _doormesh (Variables|Settings|GetOffset) false false)
  (CallFunction|SetupEditor))

(fn SetupEditor
  (bind _doorpivot (Variables|Default|GetDoorPivot))
  (bind _openangle (Variables|Settings|GetOpenAngle))
  (bind _doormesh (Variables|Default|GetDoorMesh))
  (bind _boxextent (Collision|GetComponentBounds _doormesh))
  (bind _returnvalue (* _openangle -1.0))
  (bind _relativelocation (Variables|/Script/Engine.SceneComponent|GetRelativeLocation _doorpivot))
  (bind _relativerotation (Variables|/Script/Engine.SceneComponent|GetRelativeRotation _doorpivot))
  (bind _returnvalue_2 (Math|Rotator|CombineRotators _relativerotation "0.000000,90.000000,0.000000"))
  (bind _returnvalue_3 (Math|Float|Max(Float) (.x _boxextent) (.y _boxextent)))
  (bind _returnvalue_4 (+ _relativelocation "0.000000,0.000000,1.000000"))
  (bind _returnvalue_5 (* _returnvalue_3 2.0))
  (bind _editorshape (Variables|Default|GetEditorShape)
    (:then
      (Utilities|Map|Clear (Variables|/Script/ToroCore.EditorShapeComponent|GetWireArcs _editorshape))
      (Utilities|Map|Add (Variables|/Script/ToroCore.EditorShapeComponent|GetWireArcs _editorshape) "A" (Utilities|Struct|MakeWireArcData _returnvalue_4 _returnvalue_2 (Math|Float|Min(Float) _openangle 0.0) (Math|Float|Max(Float) _openangle 0.0) _returnvalue_5 16 1.0 "(R=0.000000,G=1.000000,B=1.000000,A=1.000000)" false))
      (if (Variables|Settings|GetMultiAngle)
        (Utilities|Map|Add (Variables|/Script/ToroCore.EditorShapeComponent|GetWireArcs _editorshape) "B" (Utilities|Struct|MakeWireArcData _returnvalue_4 _returnvalue_2 (Math|Float|Min(Float) _returnvalue 0.0) (Math|Float|Max(Float) _returnvalue 0.0) _returnvalue_5 16 1.0 "(R=0.000000,G=1.000000,B=1.000000,A=1.000000)" false))))
    (:else)))